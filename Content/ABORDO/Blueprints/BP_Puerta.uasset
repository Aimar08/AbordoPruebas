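; VR door actor that the player swings by hand and that can also open or close through events.
; While grabbed, with the VRGameState status at a specific value and the hand near the Sphere, Tick yaws the actor toward the motion controller.
; Open and Close events use timelines to blend yaw toward targets.
; All rotation is clamped to symmetric limits derived from the door's starting yaw plus 90 degrees.
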(event `self.GrabComponent.OnGrabbed`
  ;[1 1 1] GestionLoc
  (set `self.loc` true))

(event `self.GrabComponent.OnDropped`
  ;[1 1 1] GestionLoc
  (set `self.loc` false))

(event `self.ReceiveBeginPlay`
  (bind (_returnvalue_roll _returnvalue_pitch _returnvalue_yaw) (`KismetMathLibrary.BreakRotator` (`SceneComponent.K2_GetComponentRotation` (`self.PROP_Door`))))
  ;[0.7728 0.3458 1] Pilla rot inicial
  (set `self.StartRot` (+ _returnvalue_yaw 90.0))
  (bind _asvrgame_state (cast `/Game/ABORDO/Blueprints/VRGameState` (`GameplayStatics.GetGameState`)))
  (add `/Game/ABORDO/Blueprints/VRGameState.status` _asvrgame_state (delegate `status_Event`)))

(event `self.ReceiveTick`
  (params (DeltaSeconds :type "Float (single-precision)"))
  (bind _startrot (`self.StartRot`))
  (bind _returnvalue (`SceneComponent.K2_GetComponentLocation` (`/Game/VRTemplate/Blueprints/GrabComponent.Motion` (`self.GrabComponent`))))
  (bind (_returnvalue_roll _returnvalue_pitch _returnvalue_yaw) (`KismetMathLibrary.BreakRotator` (`KismetMathLibrary.FindLookAtRotation` (`SceneComponent.K2_GetComponentLocation` (`self.PROP_Door`)) _returnvalue)))
  ;[0.401 0.235 0.06786] Rotar puerta
  (if (`|EnumEquality` (`self.State`) "NewEnumerator3")
    (if (< (`KismetMathLibrary.Vector_Distance` _returnvalue (`SceneComponent.K2_GetComponentLocation` (`self.Sphere`))) 39.0)
      (if (`self.loc`)
        (`self.K2_SetActorRotation` self (`KismetMathLibrary.MakeRotator` 0.0 0.0 (`KismetMathLibrary.FClamp` _returnvalue_yaw (* _startrot -1.0) _startrot)) false)))))

(event `status_Event`
  (params (PlayerController :type "/Game/ABORDO/PlayerStates Enum" :default "NewEnumerator0"))
  (set `self.State` PlayerController))

(event `Open`
  (bind _startrot (`self.StartRot`))
  (bind (_returnvalue_roll _returnvalue_pitch _returnvalue_yaw) (`KismetMathLibrary.BreakRotator` (`SceneComponent.K2_GetComponentRotation` (`self.PROP_Door`))))
  ;[1 1 1] Open
  (bind (_direction _open) (`Timeline|Timeline`)
    (:`Update`
      (`self.K2_SetActorRotation` self (`KismetMathLibrary.MakeRotator` _returnvalue_roll _returnvalue_pitch (`KismetMathLibrary.FClamp` (+ _returnvalue_yaw (* _open (- (* (`self.StartRot`) -1.0) _returnvalue_yaw))) (* _startrot -1.0) _startrot)) false))))

(event `Close`
  (bind _startrot (`self.StartRot`))
  (bind (_returnvalue_roll _returnvalue_pitch _returnvalue_yaw) (`KismetMathLibrary.BreakRotator` (`SceneComponent.K2_GetComponentRotation` (`self.PROP_Door`))))
  ;[1 1 1] Close
  (bind (_direction _open) (`Timeline|Timeline_0`)
    (:`Update`
      (`self.K2_SetActorRotation` self (`KismetMathLibrary.MakeRotator` _returnvalue_roll _returnvalue_pitch (`KismetMathLibrary.FClamp` (+ _returnvalue_yaw (* _open (- (- (`self.StartRot`) 90.0) _returnvalue_yaw))) (* _startrot -1.0) _startrot)) false))))

(fn `UserConstructionScript`)