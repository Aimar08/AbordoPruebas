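; BP_PropCocina is a grabbable VR kitchen prop that the player places on a matching target.
; Holding it ignores all collision, and dropping restores blocking.
; Overlapping the actor named by Nombre snaps it there, removes grabbing, clears its stencil highlight and destroys the target with its attachments.
; Each placement increments the VR pawn's CurrentId, calling SetEnd(false) on Dhruv's AI at six; Tick returns fallen props to their start.
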(event `self.ReceiveBeginPlay`
  (bind _staticmesh (`self.StaticMesh`))
  (set `self.begin` (`SceneComponent.K2_GetComponentLocation` _staticmesh))
  (set `self.begin1` (`KismetMathLibrary.Conv_RotatorToVector` (`SceneComponent.K2_GetComponentRotation` _staticmesh))))

(event `self.GrabComponent.OnGrabbed`
  (set `self.IsGrabbed` true)
  (`PrimitiveComponent.SetCollisionResponseToAllChannels` (`self.StaticMesh`) "ECR_Ignore"))

(event `self.GrabComponent.OnDropped`
  (set `self.IsGrabbed` false)
  (`PrimitiveComponent.SetCollisionResponseToAllChannels` (`self.StaticMesh`) "ECR_Block"))

(event `self.StaticMesh.OnComponentBeginOverlap`
  (params (OverlappedComponent :type "PrimitiveComponent Object Reference") (OtherActor :type "Actor Object Reference") (OtherComp :type "PrimitiveComponent Object Reference") (OtherBodyIndex :type Integer) (bFromSweep :type Boolean) (SweepResult :type "HitResult Structure (by ref)"))
  (bind _staticmesh (`self.StaticMesh`))
  (if (`KismetStringLibrary.EqualEqual_StrStr` (`KismetSystemLibrary.GetObjectName` OtherActor) (`self.Nombre`))
    (`ActorComponent.K2_DestroyComponent` (`self.GrabComponent`))
    (`PrimitiveComponent.SetSimulatePhysics` (`self.StaticMesh`) false)
    (`SceneComponent.K2_SetWorldLocation` _staticmesh (`self.K2_GetActorLocation` OtherActor) false true)
    (`SceneComponent.K2_SetRelativeRotation` _staticmesh (struct :`Yaw` 90.0) false false)
    (`ActorComponent.SetActive` (`self.GrabComponent`) false false)
    (`PrimitiveComponent.SetCustomDepthStencilValue` (`self.StaticMesh`) 0)
    (for _array_element (`self.GetAttachedActors` OtherActor true false)
      (`self.K2_DestroyActor` _array_element))
    (`self.K2_DestroyActor` OtherActor)
    (bind _asvr (cast `/Game/ABORDO/Blueprints/vr` (`GameplayStatics.GetPlayerPawn` 0)))
    (bind _currentid (`/Game/ABORDO/Blueprints/vr.CurrentId` _asvr))
    (`/Engine/EditorBlueprintResources/StandardMacros.IncrementInt` _currentid
      (:`  `
        (if (== _currentid 6)
          (bind _returnvalue (`GameplayStatics.GetActorOfClass` "/Game/ABORDO/Blueprints/BP_Dhruv3.BP_Dhruv3_C"))
          (bind _asai_dhru (cast `/Game/ABORDO/AI/AI_Dhru` (`AIBlueprintHelperLibrary.GetAIController` _returnvalue)))
          (`/Game/ABORDO/AI/AI_Dhru.SetEnd` _asai_dhru false))))))

(event `self.ReceiveTick`
  (params (DeltaSeconds :type "Float (single-precision)"))
  (bind _staticmesh (`self.StaticMesh`))
  (bind (_returnvalue_x _returnvalue_y _returnvalue_z) (`KismetMathLibrary.BreakVector` (`SceneComponent.K2_GetComponentLocation` _staticmesh)))
  (if (< _returnvalue_z -200.0)
    (`PrimitiveComponent.SetSimulatePhysics` _staticmesh false)
    (`SceneComponent.K2_SetWorldLocationAndRotation` _staticmesh (`self.begin`) (`KismetMathLibrary.Conv_VectorToRotator` (`self.begin1`)) false true)
    (`KismetSystemLibrary.Delay` 0.2)
    (`PrimitiveComponent.SetSimulatePhysics` _staticmesh true)))

(fn `UserConstructionScript`)