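; BP_Key is a grabbable VR key that unlocks BP_Puerta doors needing one.
; Its grab component stays inactive until ActivaLlave, and grabbing switches Sphere collision to Overlap until dropped.
; A held key overlapping such a door sets KeyUse, plays a lock sound and destroys itself; grab and use also advance the pawn's CurrentId sequence.
; Tick teleports a key fallen below the height limit back to its start, briefly suspending physics.
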(event `self.ReceiveBeginPlay`
  (bind _sphere (`self.Sphere`))
  (`ActorComponent.SetActive` (`self.GrabComponent`) false false)
  (set `self.begin` (`SceneComponent.K2_GetComponentLocation` _sphere))
  (set `self.begin1` (`KismetMathLibrary.Conv_RotatorToVector` (`SceneComponent.K2_GetComponentRotation` _sphere))))

(event `ActivaLlave`
  (`ActorComponent.SetActive` (`self.GrabComponent`) true false))

(event `self.ReceiveTick`
  (params (DeltaSeconds :type "Float (single-precision)"))
  (bind _sphere (`self.Sphere`))
  (bind (_returnvalue_x _returnvalue_y _returnvalue_z) (`KismetMathLibrary.BreakVector` (`SceneComponent.K2_GetComponentLocation` _sphere)))
  (if (< _returnvalue_z -200.0)
    (`PrimitiveComponent.SetSimulatePhysics` _sphere false)
    (`SceneComponent.K2_SetWorldLocationAndRotation` _sphere (`self.begin`) (`KismetMathLibrary.Conv_VectorToRotator` (`self.begin1`)) false true)
    (`KismetSystemLibrary.Delay` 0.2)
    (`PrimitiveComponent.SetSimulatePhysics` _sphere true)))

(event `self.GrabComponent.OnGrabbed`
  (set `self.IsGrabbed` true)
  (`PrimitiveComponent.SetCollisionResponseToAllChannels` (`self.Sphere`) "ECR_Overlap")
  (bind _asvr (cast `/Game/ABORDO/Blueprints/vr` (`GameplayStatics.GetPlayerPawn` 0)))
  (bind _currentid (`/Game/ABORDO/Blueprints/vr.CurrentId` _asvr))
  (if (== _currentid 2)
    (`/Engine/EditorBlueprintResources/StandardMacros.IncrementInt` _currentid
      (:`  `
        (`GameplayStatics.SpawnSoundAtLocation` "/Game/ABORDO/Sounds/S_Sistema2.S_Sistema2" (0.0 0.0 0.0) (struct) 1.0 1.0 0.0 null null)))))

(event `self.GrabComponent.OnDropped`
  (set `self.IsGrabbed` false)
  (`PrimitiveComponent.SetCollisionResponseToAllChannels` (`self.Sphere`) "ECR_Block"))

(event `self.Sphere.OnComponentBeginOverlap`
  (params (OverlappedComponent :type "PrimitiveComponent Object Reference") (OtherActor :type "Actor Object Reference") (OtherComp :type "PrimitiveComponent Object Reference") (OtherBodyIndex :type Integer) (bFromSweep :type Boolean) (SweepResult :type "HitResult Structure (by ref)"))
  (if (`self.IsGrabbed`)
    (bind _asbp_puerta (cast `/Game/ABORDO/Blueprints/BP_Puerta` OtherActor))
    (if (`/Game/ABORDO/Blueprints/BP_Puerta.NeedKey` _asbp_puerta)
      (set `/Game/ABORDO/Blueprints/BP_Puerta.KeyUse` true _asbp_puerta)
      (`GameplayStatics.SpawnSoundAtLocation` "/Game/ABORDO/Sounds/S_Cerradura.S_Cerradura" (0.0 0.0 0.0) (struct) 1.0 1.0 0.0 null null)
      (`self.K2_DestroyActor`)
      (bind _currentid (`/Game/ABORDO/Blueprints/vr.CurrentId` (stale `self.GrabComponent.OnGrabbed` _asvr)))
      (if (== _currentid 3)
        (`/Engine/EditorBlueprintResources/StandardMacros.IncrementInt` _currentid
          (:`  `
            (`GameplayStatics.SpawnSoundAtLocation` "/Game/ABORDO/Sounds/S_Sistema2.S_Sistema2" (0.0 0.0 0.0) (struct) 1.0 1.0 0.0 null null)))))))

(fn `UserConstructionScript`)