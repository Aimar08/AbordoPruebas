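; BP_Guide is a proximity help hint that shows its Text in a widget component to the vr player at a matching step.
; On BeginPlay it creates a WB_Help widget with that text and starts hidden.
; Sphere overlap shows the widget when the player's CurrentId equals the guide's Id, and destroys the guide when CurrentId is higher.
; Leaving the sphere hides the widget again.
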(event `self.ReceiveBeginPlay`
  (bind _widget (`self.Widget`))
  (bind _returnvalue (`|CreateWidget` "/Game/ABORDO/Widgets/WB_Help.WB_Help_C" null (`self.Text`)))
  (`WidgetComponent.SetWidget` _widget _returnvalue)
  (`SceneComponent.SetVisibility` _widget false false))

(event `self.Sphere.OnComponentBeginOverlap`
  (params (OverlappedComponent :type "PrimitiveComponent Object Reference") (OtherActor :type "Actor Object Reference") (OtherComp :type "PrimitiveComponent Object Reference") (OtherBodyIndex :type Integer) (bFromSweep :type Boolean) (SweepResult :type "HitResult Structure (by ref)"))
  (bind _id (`self.Id`))
  (bind _asvr (cast `/Game/ABORDO/Blueprints/vr` OtherActor))
  (bind _currentid (`/Game/ABORDO/Blueprints/vr.CurrentId` _asvr))
  (if (> _currentid _id)
    (`self.K2_DestroyActor`)
    (elif (== _currentid _id)
      (`SceneComponent.SetVisibility` (`self.Widget`) true false))))

(event `self.Sphere.OnComponentEndOverlap`
  (params (OverlappedComponent :type "PrimitiveComponent Object Reference") (OtherActor :type "Actor Object Reference") (OtherComp :type "PrimitiveComponent Object Reference") (OtherBodyIndex :type Integer))
  (cast `/Game/ABORDO/Blueprints/vr` OtherActor)
  (`SceneComponent.SetVisibility` (`self.Widget`) false false))

(fn `UserConstructionScript`)