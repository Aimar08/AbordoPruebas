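; VR door that the player swings by grabbing its handle, with optional key gating.
; On grab, the grab component moves to one of two mesh positions chosen by motion-controller distance, recording the side.
; Tick yaws the actor toward the nearby controller within clamped limits and tilts the handle, only in allowed VRGameState statuses.
; Open and Close events rotate the door through timelines instead.
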(event `self.GrabComponent.OnGrabbed`
  ;[1 1 1] GestionLoc
  (`self.FindNearest`)
  (set `self.isGrabing` true))

(event `FindNearest`
  (bind _grabcomponent (`self.GrabComponent`))
  (bind _motion (`/Game/VRTemplate/Blueprints/GrabComponent.Motion` (`self.GrabComponent`)))
  (bind _returnvalue (`SceneComponent.K2_GetComponentLocation` _motion))
  (if (`KismetSystemLibrary.IsValid` _motion)
    (if (> (`KismetMathLibrary.Vector_Distance` (`SceneComponent.K2_GetComponentLocation` (`self.StaticMesh1`)) _returnvalue) (`KismetMathLibrary.Vector_Distance` (`SceneComponent.K2_GetComponentLocation` (`self.StaticMesh2`)) _returnvalue))
      (set `self.GrabbedRight` false)
      (`SceneComponent.K2_SetRelativeLocation` _grabcomponent (`SceneComponent.RelativeLocation` (`self.StaticMesh1`)) false true)
      (else
        (set `self.GrabbedRight` true)
        (`SceneComponent.K2_SetRelativeLocation` _grabcomponent (`SceneComponent.RelativeLocation` (`self.StaticMesh2`)) false true)))))

(event `self.GrabComponent.OnDropped`
  ;[1 1 1] GestionLoc
  (set `self.isGrabing` false)
  (`SceneComponent.K2_SetRelativeLocation` (`self.GrabComponent`) (`self.pos`) false true)
  (`SceneComponent.K2_SetRelativeRotation` (`self.manilla`) (`KismetMathLibrary.MakeRotator` 90.0) false false))

(event `self.ReceiveBeginPlay`
  (bind (_returnvalue_roll _returnvalue_pitch _returnvalue_yaw) (`KismetMathLibrary.BreakRotator` (`SceneComponent.K2_GetComponentRotation` (`self.PropPuerta`))))
  ;[0.7728 0.3458 1] Pilla rot inicial
  (set `self.pos` (`SceneComponent.RelativeLocation` (`self.GrabComponent`)))
  (set `self.StartRot` (+ _returnvalue_yaw 90.0))
  (bind _asvrgame_state (cast `/Game/ABORDO/Blueprints/VRGameState` (`GameplayStatics.GetGameState`)))
  (add `/Game/ABORDO/Blueprints/VRGameState.status` _asvrgame_state (delegate `status_Event`)))

(event `self.ReceiveTick`
  (params (DeltaSeconds :type "Float (single-precision)"))
  (bind _state (`self.state`))
  (bind _startrot (`self.StartRot`))
  (bind _needkey (`self.NeedKey`))
  (bind _motion (`/Game/VRTemplate/Blueprints/GrabComponent.Motion` (`self.GrabComponent`)))
  (bind _returnvalue (`SceneComponent.K2_GetComponentLocation` _motion))
  (bind (_returnvalue_roll _returnvalue_pitch _returnvalue_yaw) (`KismetMathLibrary.BreakRotator` (`KismetMathLibrary.FindLookAtRotation` (`SceneComponent.K2_GetComponentLocation` (`self.PropPuerta`)) _returnvalue)))
  (bind _returnvalue_2 (`KismetMathLibrary.FClamp` _returnvalue_yaw (* _startrot -1.0) _startrot))
  ;[0.401 0.235 0.06786] Rotar puerta
  (if (or (not _needkey) (and (`self.KeyUse`) _needkey))
    (`/Engine/EditorBlueprintResources/StandardMacros.IsValid` _motion
      (:`Is Valid`
        (if (or (`|EnumEquality` _state "NewEnumerator3") (`|EnumEquality` _state "NewEnumerator0"))
          (if (< (`KismetMathLibrary.Vector_Distance` _returnvalue (`SceneComponent.K2_GetComponentLocation` (`self.GrabComponent`))) 29.0)
            (if (`self.isGrabing`)
              (if (`self.GrabbedRight`)
                (`self.K2_SetActorRotation` self (`KismetMathLibrary.MakeRotator` 0.0 0.0 (- _returnvalue_2 5.0)) false)
                (else
                  (`self.K2_SetActorRotation` self (`KismetMathLibrary.MakeRotator` 0.0 0.0 (+ _returnvalue_2 5.0)) false)))
              (`SceneComponent.K2_SetRelativeRotation` (`self.manilla`) (`KismetMathLibrary.MakeRotator` 90.0 20.0) false false)
              (else
                (`KismetSystemLibrary.PrintString` "jjjjjj")))
            (else
              (`SceneComponent.K2_SetRelativeRotation` (`self.manilla`) (`KismetMathLibrary.MakeRotator` 90.0) false false :!label _label)))
          (else
            (goto _label)))))))

(event `status_Event`
  (params (PlayerController :type "/Game/ABORDO/PlayerStates Enum" :default "NewEnumerator0"))
  (set `self.State` PlayerController))

(event `Open`
  (bind _startrot (`self.StartRot`))
  (bind (_returnvalue_roll _returnvalue_pitch _returnvalue_yaw) (`KismetMathLibrary.BreakRotator` (`SceneComponent.K2_GetComponentRotation` (`self.PropPuerta`))))
  ;[1 1 1] Open
  (bind (_direction _open) (`Timeline|Timeline`)
    (:`Update`
      (`self.K2_SetActorRotation` self (`KismetMathLibrary.MakeRotator` _returnvalue_roll _returnvalue_pitch (`KismetMathLibrary.FClamp` (+ _returnvalue_yaw (* _open (- (* (`self.StartRot`) -1.0) _returnvalue_yaw))) (* _startrot -1.0) _startrot)) false)
      (`SceneComponent.K2_SetRelativeRotation` (`self.manilla`) (`KismetMathLibrary.MakeRotator` 90.0 20.0) false false))))

(event `Close`
  (bind _startrot (`self.StartRot`))
  (bind (_returnvalue_roll _returnvalue_pitch _returnvalue_yaw) (`KismetMathLibrary.BreakRotator` (`SceneComponent.K2_GetComponentRotation` (`self.PropPuerta`))))
  ;[1 1 1] Close
  (bind (_direction _open) (`Timeline|Timeline_0`)
    (:`Update`
      (`self.K2_SetActorRotation` self (`KismetMathLibrary.MakeRotator` _returnvalue_roll _returnvalue_pitch (`KismetMathLibrary.FClamp` (+ _returnvalue_yaw (* _open (- (- (`self.StartRot`) 90.0) _returnvalue_yaw))) (* _startrot -1.0) _startrot)) false)
      (`SceneComponent.K2_SetRelativeRotation` (`self.manilla`) (`KismetMathLibrary.MakeRotator` 90.0) false false))))

(fn `UserConstructionScript`)