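; BP_Chaleco is a grabbable vest that the VR player equips on first grab.
; Grabbing sets the pawn's CurrentId, disables mesh collision, snaps the actor to the pawn and resets the mesh's custom depth stencil.
; The same grab lets the BP_Dhruv3 AI start moving through its AI_Dhru controller.
; While equipped, Tick keeps the mesh upright, following only the camera's yaw with a 90-degree offset.
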(event `self.ReceiveBeginPlay`)

(event `self.GrabComponent.OnGrabbed`
  (bind _returnvalue (`GameplayStatics.GetPlayerPawn` 0))
  (if (not (`self.equipado`))
    (set `self.equipado` true)
    (bind _asvr (cast `/Game/ABORDO/Blueprints/vr` _returnvalue))
    (set `/Game/ABORDO/Blueprints/vr.CurrentId` 1 _asvr)
    (`PrimitiveComponent.SetCollisionEnabled` (`self.StaticMesh`) "NoCollision")
    (`self.K2_AttachToActor` self _returnvalue "None" "SnapToTarget" "SnapToTarget" "KeepWorld" true)
    (set `self.Camera 0` (`/Game/ABORDO/Blueprints/vr.Camera_0` _asvr))
    (bind _returnvalue_2 (`GameplayStatics.GetActorOfClass` "/Game/ABORDO/Blueprints/BP_Dhruv3.BP_Dhruv3_C"))
    (bind _asai_dhru (cast `/Game/ABORDO/AI/AI_Dhru` (`AIBlueprintHelperLibrary.GetAIController` _returnvalue_2)))
    (`/Game/ABORDO/AI/AI_Dhru.SetCanMove` _asai_dhru true)
    (`PrimitiveComponent.SetCustomDepthStencilValue` (`self.StaticMesh`) 0)))

(event `self.ReceiveTick`
  (params (DeltaSeconds :type "Float (single-precision)"))
  (bind (_returnvalue_roll _returnvalue_pitch _returnvalue_yaw) (`KismetMathLibrary.BreakRotator` (`SceneComponent.K2_GetComponentRotation` (`self.Camera 0`))))
  (if (`self.equipado`)
    (`SceneComponent.K2_SetWorldRotation` (`self.StaticMesh`) (`KismetMathLibrary.MakeRotator` 0.0 0.0 (+ _returnvalue_yaw -90.0)) false false)))

(fn `UserConstructionScript`)